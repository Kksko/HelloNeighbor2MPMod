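; BP_Spawner is an actor that spawns a single BP_Box at its own location one second after play begins.
; A Spawned flag guards the spawn, which ignores collision and uses only the spawner's location, not its rotation or scale.
; The box is set to replicate without movement replication, with no authority check around the spawn.
; An empty pickup handler and its binding to Interactive never run.
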(event `self.ReceiveBeginPlay`
  (`KismetSystemLibrary.Delay` 1.0)
  (if (not (`self.Spawned`))
    (bind _returnvalue (`|SpawnActorFromClass` "/Game/HNMain/Blueprints/World/BP_Box.BP_Box_C" (`KismetMathLibrary.Conv_VectorToTransform` (`self.K2_GetActorLocation`)) "AlwaysSpawn" "OverrideRootScale" null null))
    (`self.SetReplicates` _returnvalue true)
    (`self.SetReplicateMovement` _returnvalue false)
    (set `self.Spawned` true)))

(event `O MAMAAAAAAAA`)

(fn `UserConstructionScript`)