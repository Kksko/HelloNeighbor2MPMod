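; BP_Input is a mod actor that provides keyboard access to the spawner menu.
; On BeginPlay it adds a hidden BPW_SpawnerMain widget to the viewport, then after a short delay enables input through SK_Quentin's player controller and spawns a LevelEditorCamera.
; Y toggles the menu, mouse cursor and input mode through a FlipFlop.
; Unconnected leftover nodes reference car entry and storm events but never run.
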(event `self.ReceiveBeginPlay`
  (bind _returnvalue (`|CreateWidget` "/Game/Mod/Spawner/BPW_SpawnerMain.BPW_SpawnerMain_C"))
  (`UserWidget.AddToViewport` _returnvalue 10000)
  (`Widget.SetVisibility` _returnvalue "Hidden")
  (`KismetSystemLibrary.Delay` 1.0)
  (bind _outactors (`GameplayStatics.GetAllActorsOfClass` "/Game/HNMain/Characters/Player/Quentin/SK_Quentin.SK_Quentin_C"))
  (bind _asplayer_controller (cast `PlayerController` (`Pawn.GetController` (`|GetArrayItem` _outactors))))
  (set `self.PC` _asplayer_controller)
  (`self.EnableInput` _asplayer_controller)
  (`|SpawnActorFromClass` "/Game/Mod/LevelEditor/LevelEditorCamera.LevelEditorCamera_C" (`KismetMathLibrary.MakeTransform` (0.0 0.0 0.0)) "Undefined" "OverrideRootScale" null null))

(event `Key|Y`
  (params (Key :type "Key Structure"))
  (bind _pc (`self.PC`))
  (bind _pc_2 (`self.PC`))
  (:`Pressed`
    (`/Engine/EditorBlueprintResources/StandardMacros.FlipFlop`
      (:`A`
        (`Widget.SetVisibility` (stale `self.ReceiveBeginPlay` _returnvalue) "Visible")
        (set `PlayerController.bShowMouseCursor` true _pc_2)
        (`WidgetBlueprintLibrary.SetInputMode_GameAndUIEx` _pc_2 (stale `self.ReceiveBeginPlay` _returnvalue)))
      (:`B`
        (`Widget.SetVisibility` (stale `self.ReceiveBeginPlay` _returnvalue) "Hidden")
        (set `PlayerController.bShowMouseCursor` false _pc)
        (`WidgetBlueprintLibrary.SetInputMode_GameOnly` _pc)))))

(fn `UserConstructionScript`)