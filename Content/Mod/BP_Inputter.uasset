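; Mod input relay actor that forwards keyboard and mouse controls to its referenced Quent character.
; It enables input via Quent's controller after BeginPlay, then handles movement, jump, run, inventory, action and mouse-button keys only off the server.
; Tick writes mouse axes and calls Quent's Inputs every frame.
; For locally controlled Quent, I loads map sublevel instances once with staggered delays, and U moves it to another SK_Quentin.
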(event `Key|D` :consume false
  (params (Key :type "Key Structure"))
  (bind _quent (`self.Quent`))
  (:`Pressed`
    (if (not (`KismetSystemLibrary.IsServer`))
      (set `/Game/HNMain/Characters/Player/Quentin/SK_Quentin.Right` true _quent)
      (`/Game/HNMain/Characters/Player/Quentin/SK_QuentinM.InputInventoryNext` _quent)))
  (:`Released`
    (if (not (`KismetSystemLibrary.IsServer`))
      (set `/Game/HNMain/Characters/Player/Quentin/SK_Quentin.Right` false _quent)
      (`/Game/HNMain/Characters/Player/Quentin/SK_QuentinM.InputInventoryPrev` (`self.Quent`)))))

(event `Key|A` :consume false
  (params (Key :type "Key Structure"))
  (bind _quent (`self.Quent`))
  (:`Pressed`
    (if (not (`KismetSystemLibrary.IsServer`))
      (set `/Game/HNMain/Characters/Player/Quentin/SK_Quentin.Left` true _quent)))
  (:`Released`
    (if (not (`KismetSystemLibrary.IsServer`))
      (set `/Game/HNMain/Characters/Player/Quentin/SK_Quentin.Left` false _quent))))

(event `self.ReceiveBeginPlay`
  (`KismetSystemLibrary.Delay` 1.0)
  (`self.EnableInput` (cast `PlayerController` (`Pawn.GetController` (`self.Quent`)) :!pure true)))

(event `self.ReceiveTick`
  (params (DeltaSeconds :type "Float (single-precision)"))
  (bind _quent (`self.Quent`))
  (set `/Game/HNMain/Characters/Player/Quentin/SK_Quentin.MouseX` (`self.GetInputAxisKeyValue`) _quent)
  (set `/Game/HNMain/Characters/Player/Quentin/SK_Quentin.MouseY` (`self.GetInputAxisKeyValue`) _quent)
  (`/Game/HNMain/Characters/Player/Quentin/SK_Quentin.Inputs` _quent))

(event `Key|S` :consume false
  (params (Key :type "Key Structure"))
  (bind _quent (`self.Quent`))
  (:`Pressed`
    (if (not (`KismetSystemLibrary.IsServer`))
      (set `/Game/HNMain/Characters/Player/Quentin/SK_Quentin.Backwards` true _quent)))
  (:`Released`
    (if (not (`KismetSystemLibrary.IsServer`))
      (set `/Game/HNMain/Characters/Player/Quentin/SK_Quentin.Backwards` false _quent))))

(event `Key|W` :consume false
  (params (Key :type "Key Structure"))
  (bind _quent (`self.Quent`))
  (:`Pressed`
    (if (not (`KismetSystemLibrary.IsServer`))
      (set `/Game/HNMain/Characters/Player/Quentin/SK_Quentin.Forward` true _quent)))
  (:`Released`
    (if (not (`KismetSystemLibrary.IsServer`))
      (set `/Game/HNMain/Characters/Player/Quentin/SK_Quentin.Forward` false _quent))))

(event `Key|Tab` :consume false
  (params (Key :type "Key Structure"))
  (bind _quent (`self.Quent`))
  (:`Pressed`
    (if (`KismetSystemLibrary.IsServer`)
      _
      (elif (`Pawn.IsLocallyControlled` (`self.Quent`))
        (`/Game/HNMain/Characters/Player/Quentin/SK_QuentinM.InputInventoryStart` _quent))))
  (:`Released`
    (if (`KismetSystemLibrary.IsServer`)
      (if (`Pawn.IsLocallyControlled` (`self.Quent`))
        _)
      (else
        (`/Game/HNMain/Characters/Player/Quentin/SK_QuentinM.InputInventoryEnd` _quent)
        (if (`Pawn.IsLocallyControlled` (`self.Quent`))
          _)))))

(event `Key|LeftShift` :consume false
  (params (Key :type "Key Structure"))
  (bind _quent (`self.Quent`))
  (:`Pressed`
    (if (not (`KismetSystemLibrary.IsServer`))
      (`/Game/HNMain/Characters/Player/Quentin/SK_QuentinM.InputRunStart` _quent)))
  (:`Released`
    (if (not (`KismetSystemLibrary.IsServer`))
      (`/Game/HNMain/Characters/Player/Quentin/SK_QuentinM.InputRunEnd` _quent))))

(event `Key|SpaceBar` :consume false
  (params (Key :type "Key Structure"))
  (bind _quent (`self.Quent`))
  (:`Pressed`
    (if (not (`KismetSystemLibrary.IsServer`))
      (`/Game/HNMain/Characters/Player/Quentin/SK_QuentinM.InputJumpStart` _quent)))
  (:`Released`
    (if (not (`KismetSystemLibrary.IsServer`))
      (`/Game/HNMain/Characters/Player/Quentin/SK_QuentinM.InputJumpEnd` _quent))))

(event `Key|Escape` :consume false
  (params (Key :type "Key Structure"))
  (:`Pressed`
    (if (not (`KismetSystemLibrary.IsServer`))
      (`/Game/HNMain/Characters/Player/Quentin/SK_QuentinM.InputMenu` (`self.Quent`)))))

(event `Key|LeftMouseButton` :consume false
  (params (Key :type "Key Structure"))
  (bind _quent (`self.Quent`))
  (:`Pressed`
    (if (not (`KismetSystemLibrary.IsServer`))
      (`/Game/HNMain/Characters/Player/Quentin/SK_QuentinM.InputApplyStart` _quent)))
  (:`Released`
    (if (not (`KismetSystemLibrary.IsServer`))
      (`/Game/HNMain/Characters/Player/Quentin/SK_QuentinM.InputApplyEnd` _quent))))

(event `Key|E` :consume false
  (params (Key :type "Key Structure"))
  (bind _quent (`self.Quent`))
  (:`Pressed`
    (if (not (`KismetSystemLibrary.IsServer`))
      (`/Game/HNMain/Characters/Player/Quentin/SK_QuentinM.InputActionStart` _quent)))
  (:`Released`
    (if (`KismetSystemLibrary.IsServer`)
      (if (`Pawn.IsLocallyControlled` (`self.Quent`))
        _)
      (else
        (`/Game/HNMain/Characters/Player/Quentin/SK_QuentinM.InputActionEnd` _quent)
        (if (`Pawn.IsLocallyControlled` (`self.Quent`))
          _)))))

(event `Key|RightMouseButton` :consume false
  (params (Key :type "Key Structure"))
  (bind _quent (`self.Quent`))
  (:`Pressed`
    (if (not (`KismetSystemLibrary.IsServer`))
      (`/Game/HNMain/Characters/Player/Quentin/SK_QuentinM.InputThrowStart` _quent)))
  (:`Released`
    (if (`KismetSystemLibrary.IsServer`)
      (if (`Pawn.IsLocallyControlled` (`self.Quent`))
        _)
      (else
        (`/Game/HNMain/Characters/Player/Quentin/SK_QuentinM.InputThrowEnd` _quent)
        (if (`Pawn.IsLocallyControlled` (`self.Quent`))
          _)))))

(event `Key|I`
  (params (Key :type "Key Structure"))
  (:`Pressed`
    (if (`Pawn.IsLocallyControlled` (`self.Quent`))
      (`/Engine/EditorBlueprintResources/StandardMacros.DoOnce` false
        (:`Completed`
          (`|ExecutionSequence`
            (:`then_0`
              (`LevelStreamingDynamic.LoadLevelInstance` "Cutscenes_Main"))
            (:`then_1`
              (`KismetSystemLibrary.Delay` 2.0)
              (`LevelStreamingDynamic.LoadLevelInstance` "Decals_Main"))
            (:`then_2`
              (`KismetSystemLibrary.Delay` 4.0)
              (`LevelStreamingDynamic.LoadLevelInstance` "EnvironmentDecoration_Main"))
            (:`then_3`
              (`KismetSystemLibrary.Delay` 12.0)
              (`LevelStreamingDynamic.LoadLevelInstance` "InteractiveObjects_Main"))
            (:`then_4`
              (`KismetSystemLibrary.Delay` 16.0)
              (`LevelStreamingDynamic.LoadLevelInstance` "LandscapeFoliage_Main"))
            (:`then_5`
              (`KismetSystemLibrary.Delay` 35.0)
              (`LevelStreamingDynamic.LoadLevelInstance` "Lighting_Main"))
            (:`then_6`
              (`KismetSystemLibrary.Delay` 40.0)
              (`LevelStreamingDynamic.LoadLevelInstance` "MainGeometry_Main"))
            (:`then_7`
              (`KismetSystemLibrary.Delay` 43.0)
              (`LevelStreamingDynamic.LoadLevelInstance` "Particles_Main"))
            (:`then_8`
              (`LevelStreamingDynamic.LoadLevelInstance` "SoundVolumes_Main"))
            (:`then_9`
              (`LevelStreamingDynamic.LoadLevelInstance` "Cutscenes_Main"))))))))

(event `Key|U` :consume false
  (params (Key :type "Key Structure"))
  (:`Pressed`
    (if (`Pawn.IsLocallyControlled` (`self.Quent`))
      (bind _outactors (`GameplayStatics.GetAllActorsOfClass` "/Game/HNMain/Characters/Player/Quentin/SK_Quentin.SK_Quentin_C"))
      (for _array_element _outactors
        (if (not (== _array_element (`self.Quent`)))
          (`self.K2_SetActorLocation` (`self.Quent`) (`self.K2_GetActorLocation` _array_element) false false))))))

(fn `UserConstructionScript`)