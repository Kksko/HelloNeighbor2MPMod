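; BP_MapLoader is a box-triggered loader that brings in a map's sublevels as level instances, split by content type such as lighting, geometry, foliage and particles.
; An overlap on the box calls Server, which calls Multi, names that suggest replication to all clients.
; A DoOnce and Sequence stagger most loads with increasing delays.
; SoundVolumes_Main loads undelayed, and Cutscenes_Main is requested twice, both times immediately.
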(event `multi`
  (`/Engine/EditorBlueprintResources/StandardMacros.DoOnce` false
    (:`Completed`
      (`|ExecutionSequence`
        (:`then_0`
          (`LevelStreamingDynamic.LoadLevelInstance` "Cutscenes_Main"))
        (:`then_1`
          (`KismetSystemLibrary.Delay` 2.0)
          (`LevelStreamingDynamic.LoadLevelInstance` "Decals_Main"))
        (:`then_2`
          (`KismetSystemLibrary.Delay` 4.0)
          (`LevelStreamingDynamic.LoadLevelInstance` "EnvironmentDecoration_Main"))
        (:`then_3`
          (`KismetSystemLibrary.Delay` 12.0)
          (`LevelStreamingDynamic.LoadLevelInstance` "InteractiveObjects_Main"))
        (:`then_4`
          (`KismetSystemLibrary.Delay` 16.0)
          (`LevelStreamingDynamic.LoadLevelInstance` "LandscapeFoliage_Main"))
        (:`then_5`
          (`KismetSystemLibrary.Delay` 35.0)
          (`LevelStreamingDynamic.LoadLevelInstance` "Lighting_Main"))
        (:`then_6`
          (`KismetSystemLibrary.Delay` 40.0)
          (`LevelStreamingDynamic.LoadLevelInstance` "MainGeometry_Main"))
        (:`then_7`
          (`KismetSystemLibrary.Delay` 43.0)
          (`LevelStreamingDynamic.LoadLevelInstance` "Particles_Main"))
        (:`then_8`
          (`LevelStreamingDynamic.LoadLevelInstance` "SoundVolumes_Main"))
        (:`then_9`
          (`LevelStreamingDynamic.LoadLevelInstance` "Cutscenes_Main"))))))

(event `self.Box.OnComponentBeginOverlap`
  (params (OverlappedComponent :type "PrimitiveComponent Object Reference") (OtherActor :type "Actor Object Reference") (OtherComp :type "PrimitiveComponent Object Reference") (OtherBodyIndex :type Integer) (bFromSweep :type Boolean) (SweepResult :type "HitResult Structure (by ref)"))
  (`self.server`))

(event `server`
  (`self.multi`))

(fn `UserConstructionScript`)